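; BP_PuzzleGate is a gate that opens after enough items have been collected.
; Each CollectItem call increments a counter, and reaching MaxItemsCollectable triggers OpenDoor once through a DoOnce node.
; OpenDoor plays a heavy anvil drop sound and runs a timeline that slides the Door component along its local X axis, despite the track being named DoorRotation.
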(event Custom|OpenDoor
  (Audio|PlaySound2D "/Game/Game_Item/Drop/Cue/Cue_HeavyDropAnvilC14_Cue_Cue.Cue_HeavyDropAnvilC14_Cue_Cue" 1.0 1.0 0.0 0 0)
  (bind _door_rotation (Timeline|Open%20Door%20Anim Play)
    (:Update
      (Transformation|SetRelativeLocation (Variables|Default|GetDoor) (Math|Vector|MakeVector (Math|Float|Lerp 0.0 1.1e+02 _door_rotation) 0.0 0.0) false false))))

(event Custom|Collect%20Item
  (Math|Integer|IncrementInt (Variables|Default|GetcurrentItemsCollected)
    (:%20%20
      (if (>= (Variables|Default|GetcurrentItemsCollected) (Variables|Default|GetmaxItemsCollectable))
        (Utilities|FlowControl|DoOnce false
          (:Completed
            (CallFunction|OpenDoor)))))))

(fn ConstructionScript)